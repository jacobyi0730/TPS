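; BP_Unit1 is a test unit actor in InterfaceTest that reacts to a player name call and to hits.
; On BeginPlay it finds BP_TPSPlayer and binds CallName to its FCallName event dispatcher, so a broadcast prints the unit's display name through PrintMyName.
; OnMyHit turns on physics simulation for SphereCollision and applies the supplied force to it.
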(event `self.ReceiveBeginPlay`
  (bind _returnvalue (`GameplayStatics.GetActorOfClass` "/Game/Blueprints/BP_TPSPlayer.BP_TPSPlayer_C"))
  (add `/Game/Blueprints/BP_TPSPlayer.FCallName` _returnvalue (delegate `CallName`)))

(event `CallName`
  (`self.PrintMyName`))

(event `/Game/InterfaceTest/BI_Unit.OnMyHit`
  (params (Force :type "Vector Structure"))
  (bind _spherecollision (`self.SphereCollision`))
  (`PrimitiveComponent.SetSimulatePhysics` _spherecollision true)
  (`PrimitiveComponent.AddForce` _spherecollision Force "None" false))

(event `/Game/InterfaceTest/BI_Unit.PrintMyName`
  (`KismetSystemLibrary.PrintString` (`KismetSystemLibrary.GetDisplayName` self)))

(fn `UserConstructionScript`)